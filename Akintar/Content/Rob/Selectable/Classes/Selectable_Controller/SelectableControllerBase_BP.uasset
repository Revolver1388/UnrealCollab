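; Base Blueprint for a selectable, AI-movable pawn that shows hover and selection feedback.
; Cursor-over events on the static mesh swap between base and highlight materials while it is unselected.
; Select and Deselect set the selection flag, change the material and toggle a particle system.
; RightClick sends the pawn to the hit location with AI MoveTo and prints whether it arrived or failed.
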(event `self.StaticMesh.OnBeginCursorOver`
  (params (TouchedComponent :type "PrimitiveComponent Object Reference"))
  (if (not (`self.isSelected`))
    (`PrimitiveComponent.SetMaterial` (`self.StaticMesh`) 0 (`self.matHighlight`))))

(event `self.StaticMesh.OnEndCursorOver`
  (params (TouchedComponent :type "PrimitiveComponent Object Reference"))
  (if (not (`self.isSelected`))
    (`PrimitiveComponent.SetMaterial` (`self.StaticMesh`) 0 (`self.matBase`))))

(event `self.ReceiveBeginPlay`
  (`ActorComponent.Deactivate` (`self.ParticleSystem_Selectable`)))

(event `/Game/Rob/Selectable/Interfaces/ISelectable.Select`
  (set `self.isSelected` true)
  (`PrimitiveComponent.SetMaterial` (`self.StaticMesh`) 0 (`self.matSelect`))
  (`ActorComponent.Activate` (`self.ParticleSystem_Selectable`) false))

(event `/Game/Rob/Selectable/Interfaces/ISelectable.Deselect`
  (set `self.isSelected` false)
  (`PrimitiveComponent.SetMaterial` (`self.StaticMesh`) 0 (`self.matBase`))
  (`ActorComponent.Deactivate` (`self.ParticleSystem_Selectable`)))

(event `/Game/Rob/Selectable/Interfaces/ISelectable.RightClick`
  (params (hit :type "HitResult Structure"))
  (`|AIMoveTo` self (`.Location` (`GameplayStatics.BreakHitResult` hit)) null (`self.acceptanceRadiusAI`)
    (:`OnSuccess`
      (`KismetSystemLibrary.PrintText` "AI move complete" true true (struct :`G` 1.0 :`B` 0.142064 :`A` 1.0)))
    (:`OnFail`
      (`KismetSystemLibrary.PrintText` "AI Couldn't reach" true true (struct :`R` 1.0 :`B` 0.028928 :`A` 1.0)))))

(fn `UserConstructionScript`)