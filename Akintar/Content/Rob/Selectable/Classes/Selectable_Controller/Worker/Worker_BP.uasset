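; Selectable worker unit that gathers resources and hauls them to storage on right-click orders.
; Right-clicking a Resource_BP starts a chain of custom events: AI move to it, gather a unit per second until over capacity, deposit at NearestStorage, then return.
; Right-clicking elsewhere clears the job and moves the worker to that point.
; NearestStorage and CurrentResourceType are only read here, and debug text reports progress.
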(event `/Game/Rob/Selectable/Interfaces/ISelectable.RightClick`
  (params (hit :type "HitResult Structure"))
  (bind (_bblockinghit _binitialoverlap _time _distance _location _impactpoint _normal _impactnormal _physmat _hitactor) (`GameplayStatics.BreakHitResult` hit))
  ;[1 1 1] ISelectable
  (bind _asresource_bp (cast `/Game/Rob/Selectable/Classes/NoneSelectable/Resource/Resource_BP` _hitactor)
    (:`then`
      (set `self.currentResource` _asresource_bp)
      (set `self.isWorking` true)
      (`self.CustomEvent_MoveTo`))
    (:`CastFailed`
      (set `self.currentResource` null)
      (set `self.isWorking` false)
      (`|AIMoveTo` self _location null
        (:`OnSuccess`
          (`KismetSystemLibrary.PrintText` "AI move complete" true true (struct :`G` 1.0 :`B` 0.142064 :`A` 1.0)))
        (:`OnFail`
          (`KismetSystemLibrary.PrintText` "AI Couldn't reach" true true (struct :`R` 1.0 :`B` 0.028928 :`A` 1.0)))))))

(event `CustomEvent_MoveTo`
  ;[1 1 1] MoveTo
  (`|AIMoveTo` self (0.0 0.0 0.0) (`self.currentResource`)
    (:`OnSuccess`
      (`KismetSystemLibrary.PrintText` "AI move complete" true true (struct :`G` 1.0 :`B` 0.142064 :`A` 1.0))
      (if (`self.isWorking`)
        (`self.CustomEvent_Gather`)))
    (:`OnFail`
      (`KismetSystemLibrary.PrintText` "AI Couldn't reach" true true (struct :`R` 1.0 :`B` 0.028928 :`A` 1.0))
      (set `self.currentResource` null))))

(event `CustomEvent_Gather`
  ;[1 1 1] Gather
  (`KismetSystemLibrary.Delay` 1.0)
  (`KismetSystemLibrary.PrintText` (`KismetTextLibrary.Conv_StringToText` (`KismetStringLibrary.Concat_StrStr` "Got" (`|GetEnumeratorNameAsString` (`self.currentResourceType`)))) true true (struct :`G` 1.0 :`A` 1.0) 0.5)
  (`/Engine/EditorBlueprintResources/StandardMacros.IncrementInt` (`self.currentCarrying`)
    (:`  `
      (if (<= (`self.currentCarrying`) (`self.carryingCapacity`))
        (`self.CustomEvent_Gather`)
        (else
          (`self.CustomEvent_MoveFrom`))))))

(event `CustomEvent_MoveFrom`
  ;[1 1 1] MoveFrom
  (`|AIMoveTo` self (0.0 0.0 0.0) (`self.nearestStorage`)
    (:`OnSuccess`
      (`KismetSystemLibrary.PrintText` "AI move complete" true true (struct :`G` 1.0 :`B` 0.142064 :`A` 1.0))
      (`/Game/Rob/Selectable/Classes/Selectable_Actor/Storage_BP.SetResource` (`self.nearestStorage`) (`self.currentResourceType`) (`self.currentCarrying`))
      (set `self.currentCarrying` 0)
      (`self.CustomEvent_MoveTo`))
    (:`OnFail`
      (`KismetSystemLibrary.PrintText` "AI Couldn't reach" true true (struct :`R` 1.0 :`B` 0.028928 :`A` 1.0)))))

(fn `UserConstructionScript`
  (`parent.UserConstructionScript`))