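; Selectable unit Blueprint that responds to right-click orders by moving or engaging units of a differing allegiance.
; A right-click on a non-selectable moves it to that point; an ally only prints a debug message.
; An enemy becomes CurrentTarget, starting an AI MoveTo and attack loop with a delay, repeating while the target stays valid.
; Attacks are placeholder prints without damage, and fire even when the move fails.
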(event `/Game/Rob/Selectable/Interfaces/ISelectable.RightClick`
  (params (hit :type "HitResult Structure"))
  (bind (_bblockinghit _binitialoverlap _time _distance _location _impactpoint _normal _impactnormal _physmat _hitactor) (`GameplayStatics.BreakHitResult` hit))
  ;[1 1 1] override right click
  (if (`KismetSystemLibrary.DoesImplementInterface` _hitactor "/Game/Rob/Selectable/Interfaces/ISelectable.ISelectable_C")
    (bind _asiselectable (cast `/Game/Rob/Selectable/Interfaces/ISelectable` _hitactor))
    (bind _unitallegiance (`/Game/Rob/Selectable/Interfaces/ISelectable.GetUnitAllegiance` _asiselectable))
    (bind _isenemy (`self.CheckAllegiance` _unitallegiance))
    (if _isenemy
      (`KismetSystemLibrary.PrintString` "Is Enemy" true true (struct :`R` 1.0 :`G` 0.187233 :`B` 0.207129 :`A` 1.0))
      (set `self.currentTarget` _hitactor)
      (set `self.isCombat` true)
      (`self.CustomEvent_MoveToTarget`)
      (else
        (`KismetSystemLibrary.PrintString` "Is ALly" true true (struct :`R` 0.191449 :`G` 1.0 :`B` 0.301933 :`A` 1.0))))
    (else
      (`self.CustomEvent_MoveToLocation` _location))))

(event `CustomEvent_MoveToTarget`
  ;[1 1 1] move to target
  (`|AIMoveTo` self (0.0 0.0 0.0) (`self.currentTarget`) (`self.attackRadius`)
    (:`OnSuccess`
      (`KismetSystemLibrary.PrintText` "AI move complete" true true (struct :`G` 1.0 :`B` 0.142064 :`A` 1.0)))
    (:`OnFail`
      (`KismetSystemLibrary.PrintText` "AI Couldn't reach" true true (struct :`R` 1.0 :`B` 0.028928 :`A` 1.0))))
  (`self.CheckTarget`)
  (if (`self.isCombat`)
    (`self.CustomEvent_Attack`)))

(event `CustomEvent_Attack`
  ;[1 1 1] attack
  (`KismetSystemLibrary.PrintString` (`KismetStringLibrary.Concat_StrStr` (`KismetStringLibrary.Conv_NameToString` (`self.unitName`)) ": attacked"))
  (`KismetSystemLibrary.Delay` 2.0)
  (`self.CheckTarget`)
  (if (`self.isCombat`)
    (`self.CustomEvent_MoveToTarget`)))

(fn `CheckAllegiance`
  (params (checkAllegiance :type "/Game/Rob/Selectable/Data/EAllegiance Enum" :default "NewEnumerator3"))
  (returns (isEnemy :type Boolean))
  (return (`|EnumInequality` checkAllegiance (`self.allegiance`))))

(fn `CheckTarget`
  (`/Engine/EditorBlueprintResources/StandardMacros.IsValid` (`self.currentTarget`)
    (:`Is Not Valid`
      (set `self.isCombat` false))))

(fn `UserConstructionScript`
  (`parent.UserConstructionScript`))